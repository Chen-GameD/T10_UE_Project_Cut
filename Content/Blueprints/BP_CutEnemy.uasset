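; BP_CutEnemy is an enemy actor with a skeletal mesh and a hidden procedural mesh, apparently set up for mesh cutting.
; Its construction script assigns StaticMeshVar to a static mesh component, copies that geometry into the procedural mesh, then destroys the source component and hides the copy.
; CutEvent hides both the skeletal and procedural meshes; no slicing happens in this Blueprint.
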(event Custom|CutEvent
  (Rendering|SetVisibility (Variables|Default|GetSkeletalMesh) false false)
  (Rendering|SetVisibility (Variables|Default|GetProceduralMesh) false false))

(event EventBeginPlay)

(event Collision|EventActorBeginOverlap
  (params (OtherActor :type Actor%20Object%20Reference)))

(event EventTick
  (params (DeltaSeconds :type Float%20%28single-precision%29)))

(fn ConstructionScript
  (bind _staticmesh (Variables|Default|GetStaticMesh))
  (Components|StaticMesh|SetStaticMesh (Variables|Default|GetStaticMesh) (Variables|Default|GetStaticMeshVar))
  (Class|KismetProceduralMeshLibrary|CopyProceduralMeshfromStaticMeshComponent _staticmesh 0 (Variables|Default|GetProceduralMesh) false)
  (Components|DestroyComponent _staticmesh)
  (Rendering|SetVisibility (Variables|Default|GetProceduralMesh) false false))